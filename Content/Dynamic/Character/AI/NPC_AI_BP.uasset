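; NPC AI controller that runs the guard behavior tree on the PatrolData blackboard at BeginPlay.
; Perception updates from actors not tagged Enemy set the EnemyKey blackboard value to player pawn 0 when sensed, or clear it when lost.
; Each tick, it sets the controlled BP_Character to aim and shoot whenever the controller has a valid focus actor.
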(event OnTargetPerceptionUpdated(AIPerception)
  (params (Actor :type Actor%20Object%20Reference) (Stimulus :type AI%20Stimulus%20Structure))
  (CallFunction|UpdateBlackboardEnemyKey (.bsuccessfullysensed Stimulus) Actor))

(event EventBeginPlay
  (bind _blackboardcomponent (Class|AIController|UseBlackboard "/Game/Dynamic/Character/AI/PatrolData.PatrolData"))
  (AI|RunBehaviorTree "/Game/Dynamic/Character/AI/GaurdBehaviour.GaurdBehaviour")
  (Variables|Default|SetBlackboard%20Component _blackboardcomponent))

(event EventTick
  (params (DeltaSeconds :type Float%20%28single-precision%29))
  (bind _asbp_character (Utilities|Casting|CastToBP_Character (Pawn|GetControlledPawn)))
  (bind _output_get (Variables|/Game/Dynamic/Character/Behaviour/BP_Character.BP_Character_C|SetAiming _asbp_character (Utilities|IsValid (Class|AIController|GetFocusActor))))
  (Variables|/Game/Dynamic/Character/Behaviour/BP_Character.BP_Character_C|SetShooting _asbp_character _output_get))

(fn ConstructionScript)

(fn UpdateBlackboardEnemyKey
  (params (Condition :type Boolean) (self2 :type Actor%20Object%20Reference))
  (bind _blackboard_component (Variables|Default|GetBlackboard%20Component))
  (if (not (Actor|ActorHasTag self2 "Enemy"))
    (if Condition
      (AI|Components|Blackboard|SetValueasObject _blackboard_component (Variables|Default|GetEnemy%20Key) (Game|Player|GetPlayerPawn 0))
      (else
        (AI|Components|Blackboard|ClearValue _blackboard_component (Variables|Default|GetEnemy%20Key))))))