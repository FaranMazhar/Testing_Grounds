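; AI controller for patrolling guard NPCs that runs the GaurdBehaviour behavior tree on the PatrolData blackboard.
; Perception updates for actors lacking the "Enemy" tag set EnemyKey to player pawn 0 when sensed, or clear it when lost.
; Each tick, the guard's Aiming and Shooting flags follow whether the controller has a valid focus actor.
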(event OnTargetPerceptionUpdated(AIPerception)
  (params (Actor :type Actor%20Object%20Reference) (Stimulus :type AI%20Stimulus%20Structure))
  (bind _blackboard_component (Variables|Default|GetBlackboard%20Component))
  (if (not (Actor|ActorHasTag Actor "Enemy"))
    (if (.bsuccessfullysensed Stimulus)
      (AI|Components|Blackboard|SetValueasObject _blackboard_component (Variables|Default|GetEnemy%20Key) (Game|Player|GetPlayerPawn 0))
      (else
        (AI|Components|Blackboard|ClearValue _blackboard_component (Variables|Default|GetEnemy%20Key))))))

(event EventBeginPlay
  (bind _blackboardcomponent (Class|AIController|UseBlackboard "/Game/Dynamic/NPC/AI/PatrolData.PatrolData"))
  (AI|RunBehaviorTree "/Game/Dynamic/NPC/AI/GaurdBehaviour.GaurdBehaviour")
  (Variables|Default|SetBlackboard%20Component _blackboardcomponent))

(event EventTick
  (params (DeltaSeconds :type Float%20%28single-precision%29))
  (bind _aspatrolling_gaurd (Utilities|Casting|CastToPatrollingGaurd (Pawn|GetControlledPawn)))
  (bind _output_get (Variables|/Game/Dynamic/NPC/Behaviour/PatrollingGaurd.PatrollingGaurd_C|SetAiming _aspatrolling_gaurd (Utilities|IsValid (Class|AIController|GetFocusActor))))
  (Variables|/Game/Dynamic/NPC/Behaviour/PatrollingGaurd.PatrollingGaurd_C|SetShooting _aspatrolling_gaurd _output_get))

(fn ConstructionScript)